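; Warehouse package Blueprint that gives itself one of three random color types: green, blue or orange.
; The RND_Spawn event rolls a random integer, stores the result in MyType, then maps that type to MaterialRef and applies it to the first material slot of the static mesh.
; BeginPlay and the construction script are empty, and nothing in this Blueprint calls RND_Spawn.
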(event `self.ReceiveBeginPlay`)

(event `RND_Spawn`
  ;[1 1 1] Random Generator of Packaages
  (switch `int` (`KismetMathLibrary.RandomInteger` 3)
    (:`0`
      (set `self.MyType` "NewEnumerator0"))
    (:`1`
      (set `self.MyType` "NewEnumerator1"))
    (:`2`
      (set `self.MyType` "NewEnumerator2")))
  (switch `/Game/WareHouseBPs/AssetType` (`self.MyType`)
    (:`NewEnumerator0`
      (set `self.MaterialRef` "/Game/WareHouseBPs/Materials/AssetGreen.AssetGreen"))
    (:`NewEnumerator1`
      (set `self.MaterialRef` "/Game/WareHouseBPs/Materials/AssetBlue.AssetBlue"))
    (:`NewEnumerator2`
      (set `self.MaterialRef` "/Game/WareHouseBPs/Materials/AssetOrange.AssetOrange")))
  (`PrimitiveComponent.SetMaterial` (`self.StaticMeshComponent`) 0 (`self.MaterialRef`)))

(fn `UserConstructionScript`)