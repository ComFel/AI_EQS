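; Warehouse Blueprint that accepts only green packages from carriers and displays its stored stock.
; On BeginPlay it sets its warehouse type; a carrier overlapping WarehouseRange has its green package detached, is freed to carry again, and the package joins WHGreenPackages.
; InvPrint then spawns a material-matched visual for every stored package, raising each spawn point and shifting sideways on a row-count match.
; Each delivery re-runs this over the whole array without clearing earlier visuals.
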(event `self.ReceiveBeginPlay`
  ;[1 1 1] Set WH type
  (`parent.ReceiveBeginPlay`)
  (set `self.OnlyTypeWareHouse` "NewEnumerator0"))

(event `self.WarehouseRange.OnComponentBeginOverlap`
  (params (OverlappedComponent :type "PrimitiveComponent Object Reference") (OtherActor :type "Actor Object Reference") (OtherComp :type "PrimitiveComponent Object Reference") (OtherBodyIndex :type Integer) (bFromSweep :type Boolean) (SweepResult :type "HitResult Structure (by ref)"))
  ;[1 1 1] Add package from carrier to warehouse
  (bind _ascarrier (cast `/Game/WareHouseBPs/BPs/Carrier/Carrier` OtherActor))
  (bind _packagecarrying (`/Game/WareHouseBPs/BPs/Carrier/Carrier.PackageCarrying` _ascarrier))
  (bind _asgreen_package (cast `/Game/WareHouseBPs/BPs/Packages/GreenPackage` _packagecarrying))
  (`self.K2_DetachFromActor` _packagecarrying "KeepRelative" "KeepRelative" "KeepRelative")
  (set `/Game/WareHouseBPs/BPs/Carrier/Carrier.CanCarry` true _ascarrier)
  (`KismetArrayLibrary.Array_Add` (`self.WH_GreenPackages`) _asgreen_package)
  (`self.InvPrint`))

(event `self.ReceiveTick`
  (params (DeltaSeconds :type "Float (single-precision)")))

(event `InvPrint`
  (bind _cornertransdorm_location (`KismetMathLibrary.BreakTransform` (`self.CornerTransdorm`)))
  (bind _wh_greenpackages (`self.WH_GreenPackages`))
  (bind _cornertransdorm_location_2 (`KismetMathLibrary.BreakTransform` (`self.CornerTransdorm`)))
  ;[1 1 1] Set Visual ref to Warehouse
  (for _array_element _wh_greenpackages
    (bind _output_get (set `self.TotalLenght` (- (`KismetArrayLibrary.Array_Length` _wh_greenpackages) 1)))
    (bind _output_get_2 (set `self.CornerTransdorm` (`KismetMathLibrary.MakeTransform` (+ _cornertransdorm_location_2 (0.0 0.0 70.0)))))
    (bind _returnvalue (`|SpawnActorFromClass` "/Game/WareHouseBPs/BPs/Packages/InvStash.InvStash_C" _output_get_2 "Undefined" "OverrideRootScale" null null))
    (`PrimitiveComponent.SetMaterial` (`/Game/WareHouseBPs/BPs/Packages/InvStash.Inv` _returnvalue) 0 (`/Game/WareHouseBPs/BPs/Packages/PackageAssetBP.MaterialRef` _array_element))
    (bind _output_get_3 (set `self.CountRow` (+ (`self.CountRow`) 1)))
    (if (== _output_get_3 (/ _output_get (`self.NumberRow`)))
      (set `self.CornerTransdorm` (`KismetMathLibrary.MakeTransform` (+ _cornertransdorm_location (50.0 0.0 0.0)) (struct) (1.0 1.0 1.0))))))

(fn `UserConstructionScript`
  (`parent.UserConstructionScript`))