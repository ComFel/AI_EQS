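; Orange warehouse Blueprint, a child that sets its warehouse type on BeginPlay and collects orange packages delivered by carriers.
; When a Carrier holding an OrangePackage overlaps WarehouseRange, it detaches the package, sets the carrier's CanCarry flag and adds the package to WHOrangePackages.
; The remaining custom event, loop and spawn nodes are empty or disconnected leftovers, including one that references the green package array.
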(event `self.ReceiveBeginPlay`
  ;[1 1 1] Set WH type
  (`parent.ReceiveBeginPlay`)
  (set `self.OnlyTypeWareHouse` "NewEnumerator2"))

(event `self.WarehouseRange.OnComponentBeginOverlap`
  (params (OverlappedComponent :type "PrimitiveComponent Object Reference") (OtherActor :type "Actor Object Reference") (OtherComp :type "PrimitiveComponent Object Reference") (OtherBodyIndex :type Integer) (bFromSweep :type Boolean) (SweepResult :type "HitResult Structure (by ref)"))
  ;[1 1 1] Add package from carrier to warehouse
  (bind _ascarrier (cast `/Game/WareHouseBPs/BPs/Carrier/Carrier` OtherActor))
  (bind _packagecarrying (`/Game/WareHouseBPs/BPs/Carrier/Carrier.PackageCarrying` _ascarrier))
  (bind _asorange_package (cast `/Game/WareHouseBPs/BPs/Packages/OrangePackage` _packagecarrying))
  (`self.K2_DetachFromActor` _packagecarrying "KeepRelative" "KeepRelative" "KeepRelative")
  (set `/Game/WareHouseBPs/BPs/Carrier/Carrier.CanCarry` true _ascarrier)
  (`KismetArrayLibrary.Array_Add` (`self.WH_OrangePackages`) _asorange_package))

(event `self.ReceiveTick`
  (params (DeltaSeconds :type "Float (single-precision)")))

(event `CustomEvent`
  (for _array_element _
    _))

(fn `UserConstructionScript`
  (`parent.UserConstructionScript`))