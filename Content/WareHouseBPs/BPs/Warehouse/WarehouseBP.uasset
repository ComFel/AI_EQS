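; Warehouse actor tied to one package type (Green, Blue or Orange), apparently a drop point for carried packages.
; BeginPlay colors its tag mesh by type, resets drop and row counters, and calls CalculateArea, whose bounds math is unwired.
; CheckType clears CanDrop when the package type matches the warehouse's and sets it otherwise.
; Overlap and inventory-print events are stubs; the Carrier-to-typed-array storage logic is disconnected.
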(event `self.ReceiveBeginPlay`
  ;[1 1 1] Set WH type VisualReference
  (switch `/Game/WareHouseBPs/BPs/AssetType` (`self.OnlyTypeWareHouse`)
    (:`NewEnumerator0`
      (set `self.MaterialRef` "/Game/WareHouseBPs/Materials/AssetGreen.AssetGreen"))
    (:`NewEnumerator1`
      (set `self.MaterialRef` "/Game/WareHouseBPs/Materials/AssetBlue.AssetBlue"))
    (:`NewEnumerator2`
      (set `self.MaterialRef` "/Game/WareHouseBPs/Materials/AssetOrange.AssetOrange")))
  (`PrimitiveComponent.SetMaterial` (`self.TagWH`) 0 (`self.MaterialRef`))
  (set `self.canDrop` true)
  (set `self.NumberRow` 0)
  (set `self.CornerTransdorm` (`KismetMathLibrary.MakeTransform` (+ (`self.K2_GetActorLocation`) (`.BoxExtent` (`KismetSystemLibrary.GetComponentBounds` (`self.WarehouseRange`))))))
  (set `self.CountRow` 0)
  (set `self.TotalLenght` 0))

(event `self.WarehouseRange.OnComponentBeginOverlap`
  (params (OverlappedComponent :type "PrimitiveComponent Object Reference") (OtherActor :type "Actor Object Reference") (OtherComp :type "PrimitiveComponent Object Reference") (OtherBodyIndex :type Integer) (bFromSweep :type Boolean) (SweepResult :type "HitResult Structure (by ref)"))
  ;[1 1 1] Set WH Type Array
)

(event `PrintInvState`
  (for _array_element (`self.TempPackages`)
    (switch `/Game/WareHouseBPs/BPs/AssetType` (`/Game/WareHouseBPs/BPs/Packages/PackageAssetBP.MyType` _array_element))))

(event `CheckType`
  (params (NewParam :type "/Game/WareHouseBPs/BPs/Packages/PackageAssetBP Object Reference"))
  (if (`|EnumEquality` (`/Game/WareHouseBPs/BPs/Packages/PackageAssetBP.MyType` NewParam) (`self.OnlyTypeWareHouse`))
    (set `self.canDrop` false)
    (else
      (set `self.canDrop` true))))

(fn `UserConstructionScript`)