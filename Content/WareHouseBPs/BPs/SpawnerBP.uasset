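; Spawner actor that repeatedly drops PackageAssetBP packages at random X/Y points within its Range component's bounds, at the actor's own height.
; Tick runs through a Delay of CdToSpawn, which paces SpawnPackage.
; Each spawn replaces PackagesList with only the new package and prints its name.
; The CanSpawn cooldown check and the array append are disconnected, so neither runs.
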(event `self.ReceiveBeginPlay`
  (set `self.Cd_ToSpawn` (`self.Cd_ToSpawn`)))

(event `CdSpwan`
  ;[1 1 1] Cooldown for Spawn
  (bind _output_get (set `self.Cd_ToSpawn` (- (`self.Cd_ToSpawn`) 0.1)))
  (if (<= _output_get 0.0)
    (set `self.CanSpawn` true)
    (set `self.Cd_ToSpawn` (`self.Cd_ToSpawn`))))

(event `self.ReceiveTick`
  (params (DeltaSeconds :type "Float (single-precision)"))
  (`KismetSystemLibrary.Delay` (`self.Cd_ToSpawn`))
  (`self.SpawnPackage`))

(event `SpawnPackage`
  (bind (_origin _boxextent) (`KismetSystemLibrary.GetComponentBounds` (`self.Range`)))
  ;[1 1 1] Actor / Package Spawner
  (bind _returnvalue (`|SpawnActorFromClass` "/Game/WareHouseBPs/BPs/PackageAssetBP.PackageAssetBP_C" (`KismetMathLibrary.MakeTransform` (+ (`self.K2_GetActorLocation`) (`KismetMathLibrary.MakeVector` (`KismetMathLibrary.RandomFloatInRange` (* (.x _boxextent) -1.0) (.x _boxextent)) (`KismetMathLibrary.RandomFloatInRange` (* (.y _boxextent) -1.0) (.y _boxextent))))) "AlwaysSpawn" "OverrideRootScale" null null))
  (set `self.CanSpawn` false)
  ;[1 1 1] Add Package Array
  (bind _output_get (set `self.PackagesList` (`|MakeArray` _returnvalue)))
  (`KismetSystemLibrary.PrintString` (`KismetSystemLibrary.GetDisplayName` (`|GetArrayItem` _output_get)) true true (struct :`R` 1.0 :`G` 0.036361 :`A` 1.0)))

(fn `UserConstructionScript`)